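; Logic gate actor for the power cable system that powers or cuts a linked output cable based on its powered inputs.
; Poweron and PowerOff events adjust a powered-input count, then re-run the BeginPlay evaluation, which switches on gate type (AND, OR, XOR, NOT and their variants) to set the cable's IsFilling flag.
; The construction script labels the gate with its type and, for NOT, reduces the two input spheres to one repositioned sphere.
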(event EventPowerOff
  (bind _linkedoutputcable (Variables|Default|GetLinkedOutputCable))
  (bind _linkedoutputcable_2 (Variables|Default|GetLinkedOutputCable))
  (bind _linkedoutputcable_3 (Variables|Default|GetLinkedOutputCable))
  (bind _linkedoutputcable_4 (Variables|Default|GetLinkedOutputCable))
  (bind _linkedoutputcable_5 (Variables|Default|GetLinkedOutputCable))
  (bind _linkedoutputcable_6 (Variables|Default|GetLinkedOutputCable))
  (bind _linkedoutputcable_7 (Variables|Default|GetLinkedOutputCable))
  (bind _linkedoutputcable_8 (Variables|Default|GetLinkedOutputCable))
  (bind _linkedoutputcable_9 (Variables|Default|GetLinkedOutputCable))
  (bind _linkedoutputcable_10 (Variables|Default|GetLinkedOutputCable))
  (bind _linkedoutputcable_11 (Variables|Default|GetLinkedOutputCable))
  (bind _poweramount (Variables|Default|GetPowerAmount))
  (bind _linkedoutputcable_12 (Variables|Default|GetLinkedOutputCable))
  (bind _linkedoutputcable_13 (Variables|Default|GetLinkedOutputCable))
  (bind _linkedoutputcable_14 (Variables|Default|GetLinkedOutputCable))
  (Math|Integer|DecrementInt (Variables|Default|GetPowerAmount)
    (:%20%20
      (switch Utilities|FlowControl|Switch|SwitchonGates_Types (Variables|Default|GetGateType)
        (:NewEnumerator0
          ;[0.3441 0.6427 1] AND Gate. Power output if both inputs are powered
          (if (== (Variables|Default|GetPowerAmount) 2)
            (Utilities|IsValid _linkedoutputcable_13
              (:Is%20Valid
                (Variables|/Game/PowerCables/Blueprints/BP_Cable.BP_Cable_C|SetisFilling _linkedoutputcable_13 true)))
            (else
              (Utilities|IsValid _linkedoutputcable_6
                (:Is%20Valid
                  (Variables|/Game/PowerCables/Blueprints/BP_Cable.BP_Cable_C|SetisFilling _linkedoutputcable_6 false))))))
        (:NewEnumerator2
          ;[0.3441 0.6427 1] NAND Gate. Power output as long as both inputs aren't powered
          (if (!= (Variables|Default|GetPowerAmount) 2)
            (Utilities|IsValid _linkedoutputcable_14
              (:Is%20Valid
                (Variables|/Game/PowerCables/Blueprints/BP_Cable.BP_Cable_C|SetisFilling _linkedoutputcable_14 true)))
            (else
              (Utilities|IsValid _linkedoutputcable_7
                (:Is%20Valid
                  (Variables|/Game/PowerCables/Blueprints/BP_Cable.BP_Cable_C|SetisFilling _linkedoutputcable_7 false))))))
        (:NewEnumerator1
          ;[0.3441 0.6427 1] OR Gate. Power output if any input is powered
          (if (> (Variables|Default|GetPowerAmount) 0)
            (Utilities|IsValid _linkedoutputcable
              (:Is%20Valid
                (Variables|/Game/PowerCables/Blueprints/BP_Cable.BP_Cable_C|SetisFilling _linkedoutputcable true)))
            (else
              (Utilities|IsValid _linkedoutputcable_8
                (:Is%20Valid
                  (Variables|/Game/PowerCables/Blueprints/BP_Cable.BP_Cable_C|SetisFilling _linkedoutputcable_8 false))))))
        (:NewEnumerator3
          ;[0.3441 0.6427 1] XOR Gate. Power output if only one input is powered
          (if (== (Variables|Default|GetPowerAmount) 1)
            (Utilities|IsValid _linkedoutputcable_2
              (:Is%20Valid
                (Variables|/Game/PowerCables/Blueprints/BP_Cable.BP_Cable_C|SetisFilling _linkedoutputcable_2 true)))
            (else
              (Utilities|IsValid _linkedoutputcable_9
                (:Is%20Valid
                  (Variables|/Game/PowerCables/Blueprints/BP_Cable.BP_Cable_C|SetisFilling _linkedoutputcable_9 false))))))
        (:NewEnumerator5
          ;[0.3441 0.6427 1] NOR Gate. Power output if neither input is powered
          (if (== (Variables|Default|GetPowerAmount) 0)
            (Utilities|IsValid _linkedoutputcable_3
              (:Is%20Valid
                (Variables|/Game/PowerCables/Blueprints/BP_Cable.BP_Cable_C|SetisFilling _linkedoutputcable_3 true)))
            (else
              (Utilities|IsValid _linkedoutputcable_10
                (:Is%20Valid
                  (Variables|/Game/PowerCables/Blueprints/BP_Cable.BP_Cable_C|SetisFilling _linkedoutputcable_10 false))))))
        (:NewEnumerator6
          ;[0.3441 0.6427 1] XNOR Gate. Power output if neither input is powered or if both inputs are powered
          (if (or (== _poweramount 0) (== _poweramount 2))
            (Utilities|IsValid _linkedoutputcable_11
              (:Is%20Valid
                (Variables|/Game/PowerCables/Blueprints/BP_Cable.BP_Cable_C|SetisFilling _linkedoutputcable_11 true)))
            (else
              (Utilities|IsValid _linkedoutputcable_12
                (:Is%20Valid
                  (Variables|/Game/PowerCables/Blueprints/BP_Cable.BP_Cable_C|SetisFilling _linkedoutputcable_12 false))))))
        (:NewEnumerator4
          ;[0.3441 0.6427 1] NOT Gate. Power output if the input is not powered
          (if (== (Variables|Default|GetPowerAmount) 0)
            (Utilities|IsValid _linkedoutputcable_5
              (:Is%20Valid
                (Variables|/Game/PowerCables/Blueprints/BP_Cable.BP_Cable_C|SetisFilling _linkedoutputcable_5 true)))
            (else
              (Utilities|IsValid _linkedoutputcable_4
                (:Is%20Valid
                  (Variables|/Game/PowerCables/Blueprints/BP_Cable.BP_Cable_C|SetisFilling _linkedoutputcable_4 false))))))))))

(event EventPoweron
  (bind _linkedoutputcable (Variables|Default|GetLinkedOutputCable))
  (bind _linkedoutputcable_2 (Variables|Default|GetLinkedOutputCable))
  (bind _linkedoutputcable_3 (Variables|Default|GetLinkedOutputCable))
  (bind _linkedoutputcable_4 (Variables|Default|GetLinkedOutputCable))
  (bind _linkedoutputcable_5 (Variables|Default|GetLinkedOutputCable))
  (bind _linkedoutputcable_6 (Variables|Default|GetLinkedOutputCable))
  (bind _linkedoutputcable_7 (Variables|Default|GetLinkedOutputCable))
  (bind _linkedoutputcable_8 (Variables|Default|GetLinkedOutputCable))
  (bind _linkedoutputcable_9 (Variables|Default|GetLinkedOutputCable))
  (bind _linkedoutputcable_10 (Variables|Default|GetLinkedOutputCable))
  (bind _linkedoutputcable_11 (Variables|Default|GetLinkedOutputCable))
  (bind _poweramount (Variables|Default|GetPowerAmount))
  (bind _linkedoutputcable_12 (Variables|Default|GetLinkedOutputCable))
  (bind _linkedoutputcable_13 (Variables|Default|GetLinkedOutputCable))
  (bind _linkedoutputcable_14 (Variables|Default|GetLinkedOutputCable))
  (Math|Integer|IncrementInt (Variables|Default|GetPowerAmount)
    (:%20%20
      (switch Utilities|FlowControl|Switch|SwitchonGates_Types (Variables|Default|GetGateType)
        (:NewEnumerator0
          ;[0.3441 0.6427 1] AND Gate. Power output if both inputs are powered
          (if (== (Variables|Default|GetPowerAmount) 2)
            (Utilities|IsValid _linkedoutputcable_13
              (:Is%20Valid
                (Variables|/Game/PowerCables/Blueprints/BP_Cable.BP_Cable_C|SetisFilling _linkedoutputcable_13 true)))
            (else
              (Utilities|IsValid _linkedoutputcable_6
                (:Is%20Valid
                  (Variables|/Game/PowerCables/Blueprints/BP_Cable.BP_Cable_C|SetisFilling _linkedoutputcable_6 false))))))
        (:NewEnumerator2
          ;[0.3441 0.6427 1] NAND Gate. Power output as long as both inputs aren't powered
          (if (!= (Variables|Default|GetPowerAmount) 2)
            (Utilities|IsValid _linkedoutputcable_14
              (:Is%20Valid
                (Variables|/Game/PowerCables/Blueprints/BP_Cable.BP_Cable_C|SetisFilling _linkedoutputcable_14 true)))
            (else
              (Utilities|IsValid _linkedoutputcable_7
                (:Is%20Valid
                  (Variables|/Game/PowerCables/Blueprints/BP_Cable.BP_Cable_C|SetisFilling _linkedoutputcable_7 false))))))
        (:NewEnumerator1
          ;[0.3441 0.6427 1] OR Gate. Power output if any input is powered
          (if (> (Variables|Default|GetPowerAmount) 0)
            (Utilities|IsValid _linkedoutputcable
              (:Is%20Valid
                (Variables|/Game/PowerCables/Blueprints/BP_Cable.BP_Cable_C|SetisFilling _linkedoutputcable true)))
            (else
              (Utilities|IsValid _linkedoutputcable_8
                (:Is%20Valid
                  (Variables|/Game/PowerCables/Blueprints/BP_Cable.BP_Cable_C|SetisFilling _linkedoutputcable_8 false))))))
        (:NewEnumerator3
          ;[0.3441 0.6427 1] XOR Gate. Power output if only one input is powered
          (if (== (Variables|Default|GetPowerAmount) 1)
            (Utilities|IsValid _linkedoutputcable_2
              (:Is%20Valid
                (Variables|/Game/PowerCables/Blueprints/BP_Cable.BP_Cable_C|SetisFilling _linkedoutputcable_2 true)))
            (else
              (Utilities|IsValid _linkedoutputcable_9
                (:Is%20Valid
                  (Variables|/Game/PowerCables/Blueprints/BP_Cable.BP_Cable_C|SetisFilling _linkedoutputcable_9 false))))))
        (:NewEnumerator5
          ;[0.3441 0.6427 1] NOR Gate. Power output if neither input is powered
          (if (== (Variables|Default|GetPowerAmount) 0)
            (Utilities|IsValid _linkedoutputcable_3
              (:Is%20Valid
                (Variables|/Game/PowerCables/Blueprints/BP_Cable.BP_Cable_C|SetisFilling _linkedoutputcable_3 true)))
            (else
              (Utilities|IsValid _linkedoutputcable_10
                (:Is%20Valid
                  (Variables|/Game/PowerCables/Blueprints/BP_Cable.BP_Cable_C|SetisFilling _linkedoutputcable_10 false))))))
        (:NewEnumerator6
          ;[0.3441 0.6427 1] XNOR Gate. Power output if neither input is powered or if both inputs are powered
          (if (or (== _poweramount 0) (== _poweramount 2))
            (Utilities|IsValid _linkedoutputcable_11
              (:Is%20Valid
                (Variables|/Game/PowerCables/Blueprints/BP_Cable.BP_Cable_C|SetisFilling _linkedoutputcable_11 true)))
            (else
              (Utilities|IsValid _linkedoutputcable_12
                (:Is%20Valid
                  (Variables|/Game/PowerCables/Blueprints/BP_Cable.BP_Cable_C|SetisFilling _linkedoutputcable_12 false))))))
        (:NewEnumerator4
          ;[0.3441 0.6427 1] NOT Gate. Power output if the input is not powered
          (if (== (Variables|Default|GetPowerAmount) 0)
            (Utilities|IsValid _linkedoutputcable_5
              (:Is%20Valid
                (Variables|/Game/PowerCables/Blueprints/BP_Cable.BP_Cable_C|SetisFilling _linkedoutputcable_5 true)))
            (else
              (Utilities|IsValid _linkedoutputcable_4
                (:Is%20Valid
                  (Variables|/Game/PowerCables/Blueprints/BP_Cable.BP_Cable_C|SetisFilling _linkedoutputcable_4 false))))))))))

(event EventBeginPlay
  (bind _linkedoutputcable (Variables|Default|GetLinkedOutputCable))
  (bind _linkedoutputcable_2 (Variables|Default|GetLinkedOutputCable))
  (bind _linkedoutputcable_3 (Variables|Default|GetLinkedOutputCable))
  (bind _linkedoutputcable_4 (Variables|Default|GetLinkedOutputCable))
  (bind _linkedoutputcable_5 (Variables|Default|GetLinkedOutputCable))
  (bind _linkedoutputcable_6 (Variables|Default|GetLinkedOutputCable))
  (bind _linkedoutputcable_7 (Variables|Default|GetLinkedOutputCable))
  (bind _linkedoutputcable_8 (Variables|Default|GetLinkedOutputCable))
  (bind _linkedoutputcable_9 (Variables|Default|GetLinkedOutputCable))
  (bind _linkedoutputcable_10 (Variables|Default|GetLinkedOutputCable))
  (bind _linkedoutputcable_11 (Variables|Default|GetLinkedOutputCable))
  (bind _poweramount (Variables|Default|GetPowerAmount))
  (bind _linkedoutputcable_12 (Variables|Default|GetLinkedOutputCable))
  (bind _linkedoutputcable_13 (Variables|Default|GetLinkedOutputCable))
  (bind _linkedoutputcable_14 (Variables|Default|GetLinkedOutputCable))
  (switch Utilities|FlowControl|Switch|SwitchonGates_Types (Variables|Default|GetGateType)
    (:NewEnumerator0
      ;[0.3441 0.6427 1] AND Gate. Power output if both inputs are powered
      (if (== (Variables|Default|GetPowerAmount) 2)
        (Utilities|IsValid _linkedoutputcable_13
          (:Is%20Valid
            (Variables|/Game/PowerCables/Blueprints/BP_Cable.BP_Cable_C|SetisFilling _linkedoutputcable_13 true)))
        (else
          (Utilities|IsValid _linkedoutputcable_6
            (:Is%20Valid
              (Variables|/Game/PowerCables/Blueprints/BP_Cable.BP_Cable_C|SetisFilling _linkedoutputcable_6 false))))))
    (:NewEnumerator2
      ;[0.3441 0.6427 1] NAND Gate. Power output as long as both inputs aren't powered
      (if (!= (Variables|Default|GetPowerAmount) 2)
        (Utilities|IsValid _linkedoutputcable_14
          (:Is%20Valid
            (Variables|/Game/PowerCables/Blueprints/BP_Cable.BP_Cable_C|SetisFilling _linkedoutputcable_14 true)))
        (else
          (Utilities|IsValid _linkedoutputcable_7
            (:Is%20Valid
              (Variables|/Game/PowerCables/Blueprints/BP_Cable.BP_Cable_C|SetisFilling _linkedoutputcable_7 false))))))
    (:NewEnumerator1
      ;[0.3441 0.6427 1] OR Gate. Power output if any input is powered
      (if (> (Variables|Default|GetPowerAmount) 0)
        (Utilities|IsValid _linkedoutputcable
          (:Is%20Valid
            (Variables|/Game/PowerCables/Blueprints/BP_Cable.BP_Cable_C|SetisFilling _linkedoutputcable true)))
        (else
          (Utilities|IsValid _linkedoutputcable_8
            (:Is%20Valid
              (Variables|/Game/PowerCables/Blueprints/BP_Cable.BP_Cable_C|SetisFilling _linkedoutputcable_8 false))))))
    (:NewEnumerator3
      ;[0.3441 0.6427 1] XOR Gate. Power output if only one input is powered
      (if (== (Variables|Default|GetPowerAmount) 1)
        (Utilities|IsValid _linkedoutputcable_2
          (:Is%20Valid
            (Variables|/Game/PowerCables/Blueprints/BP_Cable.BP_Cable_C|SetisFilling _linkedoutputcable_2 true)))
        (else
          (Utilities|IsValid _linkedoutputcable_9
            (:Is%20Valid
              (Variables|/Game/PowerCables/Blueprints/BP_Cable.BP_Cable_C|SetisFilling _linkedoutputcable_9 false))))))
    (:NewEnumerator5
      ;[0.3441 0.6427 1] NOR Gate. Power output if neither input is powered
      (if (== (Variables|Default|GetPowerAmount) 0)
        (Utilities|IsValid _linkedoutputcable_3
          (:Is%20Valid
            (Variables|/Game/PowerCables/Blueprints/BP_Cable.BP_Cable_C|SetisFilling _linkedoutputcable_3 true)))
        (else
          (Utilities|IsValid _linkedoutputcable_10
            (:Is%20Valid
              (Variables|/Game/PowerCables/Blueprints/BP_Cable.BP_Cable_C|SetisFilling _linkedoutputcable_10 false))))))
    (:NewEnumerator6
      ;[0.3441 0.6427 1] XNOR Gate. Power output if neither input is powered or if both inputs are powered
      (if (or (== _poweramount 0) (== _poweramount 2))
        (Utilities|IsValid _linkedoutputcable_11
          (:Is%20Valid
            (Variables|/Game/PowerCables/Blueprints/BP_Cable.BP_Cable_C|SetisFilling _linkedoutputcable_11 true)))
        (else
          (Utilities|IsValid _linkedoutputcable_12
            (:Is%20Valid
              (Variables|/Game/PowerCables/Blueprints/BP_Cable.BP_Cable_C|SetisFilling _linkedoutputcable_12 false))))))
    (:NewEnumerator4
      ;[0.3441 0.6427 1] NOT Gate. Power output if the input is not powered
      (if (== (Variables|Default|GetPowerAmount) 0)
        (Utilities|IsValid _linkedoutputcable_5
          (:Is%20Valid
            (Variables|/Game/PowerCables/Blueprints/BP_Cable.BP_Cable_C|SetisFilling _linkedoutputcable_5 true)))
        (else
          (Utilities|IsValid _linkedoutputcable_4
            (:Is%20Valid
              (Variables|/Game/PowerCables/Blueprints/BP_Cable.BP_Cable_C|SetisFilling _linkedoutputcable_4 false))))))))

(fn ConstructionScript
  (Rendering|Components|TextRender|SetText (Variables|Default|GetText) (Utilities|Text|ToText(String) (Utilities|String|EnumtoString (Variables|Default|GetGateType))))
  (if (Utilities|Enum|Equal(Enum) (Variables|Default|GetGateType) "NewEnumerator4")
    (Components|DestroyComponent (Variables|Default|GetSphereRight))
    (Transformation|SetRelativeLocationAndRotation (Variables|Default|GetSphereLeft) "50.000000,0.000000,10.000000" "0, 0, 0" false false)))