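; BP_Door is a powered door that swings open when powered on and returns to zero rotation when powered off.
; Each power event caches the door's current relative rotation, stops the opposing timeline and plays its own from the start.
; The timelines linearly ease from that cached rotation to the open or closed target, so an interrupted swing reverses from its current angle.
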(event EventPoweron
  (Variables|Default|SetInitialRotation (Variables|/Script/Engine.SceneComponent|GetRelativeRotation (Variables|Default|GetDoor)))
  (Utilities|FlowControl|Sequence
    (:then_0
      (bind _alpha (Timeline|Timeline_0 Stop)
        (:Update
          (Transformation|SetRelativeRotation (Variables|Default|GetDoor) (Math|Interpolation|Ease :Function "Linear" :Alpha _alpha :A (Variables|Default|GetInitialRotation)) false false))))
    (:then_1
      (bind _alpha_2 (Timeline|Timeline PlayFromStart)
        (:Update
          (Transformation|SetRelativeRotation (Variables|Default|GetDoor) (Math|Interpolation|Ease "Linear" _alpha_2 (Variables|Default|GetInitialRotation) "0.000000,-90.000000,0.000000" true) false false))))))

(event EventPowerOff
  (Variables|Default|SetInitialRotation (Variables|/Script/Engine.SceneComponent|GetRelativeRotation (Variables|Default|GetDoor)))
  (Utilities|FlowControl|Sequence
    (:then_0
      (bind _alpha (Timeline|Timeline Stop)
        (:Update
          (Transformation|SetRelativeRotation (Variables|Default|GetDoor) (Math|Interpolation|Ease "Linear" _alpha (Variables|Default|GetInitialRotation) "0.000000,-90.000000,0.000000" true) false false))))
    (:then_1
      (bind _alpha_2 (Timeline|Timeline_0 PlayFromStart)
        (:Update
          (Transformation|SetRelativeRotation (Variables|Default|GetDoor) (Math|Interpolation|Ease :Function "Linear" :Alpha _alpha_2 :A (Variables|Default|GetInitialRotation)) false false))))))

(fn ConstructionScript)