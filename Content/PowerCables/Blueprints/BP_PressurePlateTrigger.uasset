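; Pressure plate actor that powers a linked cable when an actor implementing BI_WeightedObject overlaps its box.
; ButtonOn sets the cable's IsFilling, swaps the plate material, plays a click and lowers the plate with a timeline.
; ButtonOff reverses this, but its end-overlap logic is disconnected, so stepping off never releases the plate or decrements the occupant count.
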(event OnComponentBeginOverlap(Box)
  (params (OverlappedComponent :type Primitive%20Component%20Object%20Reference) (OtherActor :type Actor%20Object%20Reference) (OtherComp :type Primitive%20Component%20Object%20Reference) (OtherBodyIndex :type Integer) (bFromSweep :type Boolean) (SweepResult :type Hit%20Result%20Structure%20%28by%20ref%29))
  ;[1 1 1] Player Steps on pressure plate
  (if (Utilities|DoesObjectImplementInterface OtherActor "/Game/PowerCables/Interfaces/BI_WeightedObject.BI_WeightedObject_C")
    (if (and (Variables|Non-Tweakable|GetisActivated) (== (Variables|Default|GetActorsOnButton) 0))
      _
      (else
        (CallFunction|Buttonon)))
    (Math|Integer|IncrementInt (Variables|Default|GetActorsOnButton))))

(event OnComponentEndOverlap(Box)
  (params (OverlappedComponent :type Primitive%20Component%20Object%20Reference) (OtherActor :type Actor%20Object%20Reference) (OtherComp :type Primitive%20Component%20Object%20Reference) (OtherBodyIndex :type Integer))
  ;[1 1 1] Player Steps off pressure plate
)

(event Custom|ButtonOff
  (bind _linkedcable (Variables|Tweakable|GetLinkedCable))
  (bind _pressureplate (Variables|Default|GetPressurePlate))
  ;[1 1 1] Power Off
  (Variables|Non-Tweakable|SetisActivated false)
  (Audio|PlaySoundatLocation "/Engine/VREditor/Sounds/UI/Camera_Shutter.Camera_Shutter" (Transformation|GetActorLocation) "0, 0, 0" 0.5 1.0 0.0 "/Game/Demo/Audio/DefaultAttenuation.DefaultAttenuation" 0 0 0)
  (Rendering|Material|SetMaterial (Variables|Default|GetPressurePlate) 0 (Variables|Tweakable|GetOffMaterial))
  (Utilities|IsValid _linkedcable
    (:Is%20Valid
      (Variables|/Game/PowerCables/Blueprints/BP_Cable.BP_Cable_C|SetisFilling _linkedcable false))
    (:Is%20Not%20Valid
      _))
  ;[0.4383 0.6818 1] Handle Button Animation
  (Utilities|FlowControl|Sequence
    (:then_0
      (bind _alpha (Timeline|Timeline Stop)
        (:Update
          (Transformation|SetRelativeLocation _pressureplate (Math|Interpolation|Ease :Function "Linear" :Alpha _alpha :A "0.000000,0.000000,4.000000") false false))))
    (:then_1
      (bind _alpha_2 (Timeline|Timeline_0 PlayFromStart)
        (:Update
          (Transformation|SetRelativeLocation _pressureplate (Math|Interpolation|Ease :Function "Linear" :Alpha _alpha_2 :B "0.000000,0.000000,4.000000") false false))))))

(event Custom|ButtonOn
  (bind _linkedcable (Variables|Tweakable|GetLinkedCable))
  (bind _pressureplate (Variables|Default|GetPressurePlate))
  ;[1 1 1] Power On
  (Variables|Non-Tweakable|SetisActivated true)
  (Audio|PlaySoundatLocation "/Engine/VREditor/Sounds/UI/Click_on_Button.Click_on_Button" (Transformation|GetActorLocation) "0, 0, 0" 0.7 1.0 0.0 "/Game/Demo/Audio/DefaultAttenuation.DefaultAttenuation" 0 0 0)
  (Rendering|Material|SetMaterial (Variables|Default|GetPressurePlate) 0 (Variables|Tweakable|GetOnMaterial))
  (Utilities|IsValid _linkedcable
    (:Is%20Valid
      (Variables|/Game/PowerCables/Blueprints/BP_Cable.BP_Cable_C|SetisFilling _linkedcable true))
    (:Is%20Not%20Valid
      _))
  ;[0.4383 0.6818 1] Handle Button Animation
  (Utilities|FlowControl|Sequence
    (:then_0
      (bind _alpha (Timeline|Timeline_0 Stop)
        (:Update
          (Transformation|SetRelativeLocation _pressureplate (Math|Interpolation|Ease :Function "Linear" :Alpha _alpha :B "0.000000,0.000000,4.000000") false false))))
    (:then_1
      (bind _alpha_2 (Timeline|Timeline PlayFromStart)
        (:Update
          (Transformation|SetRelativeLocation _pressureplate (Math|Interpolation|Ease :Function "Linear" :Alpha _alpha_2 :A "0.000000,0.000000,4.000000") false false))))))

(fn ConstructionScript)